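; Player character Blueprint with first-person-style movement and look, running, a note inventory and a scripted torch burnout.
; Axis inputs drive movement and controller rotation, while the Run action swaps the walk speed.
; The N key flip-flops the NoteInventory widget, switching cursor visibility and input mode.
; Overlapping any TriggerBox starts a delayed flicker of the point light, then destroys it and the cylinder, meant for entering the cavern.
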(event `NoteInvToggle`
  (bind _returnvalue (`GameplayStatics.GetPlayerController` 0))
  (bind _returnvalue_2 (`GameplayStatics.GetPlayerController` 0))
  ;[1 1 1] Note Inventory
  (`/Engine/EditorBlueprintResources/StandardMacros.FlipFlop`
    (:`A`
      (bind _returnvalue_3 (`|CreateWidget` "/Game/Blueprints/NoteInventory.NoteInventory_C" (`GameplayStatics.GetPlayerController` 0)))
      (bind _output_get (set `self.Note_Inv` _returnvalue_3))
      (`UserWidget.AddToViewport` _output_get 0)
      (set `PlayerController.bShowMouseCursor` true _returnvalue)
      (`WidgetBlueprintLibrary.SetInputMode_GameAndUIEx` _returnvalue (`self.Note_Inv`) "DoNotLock" false))
    (:`B`
      (`Widget.RemoveFromParent` (`self.Note_Inv`))
      (set `PlayerController.bShowMouseCursor` false _returnvalue_2)
      (`WidgetBlueprintLibrary.SetInputMode_GameOnly` _returnvalue_2))))

(event `InputAxis|Rotate_Left/Right`
  (params (AxisValue :type "Float (single-precision)"))
  ;[1 1 1] Movement
  ;;[1 1 1] Look up/down/left/right
  (`self.AddControllerYawInput` AxisValue))

(event `InputAxis|Forward/Backward`
  (params (AxisValue :type "Float (single-precision)"))
  ;[1 1 1] Movement
  ;;[1 1 1] Move for/back/left/right
  (`self.AddMovementInput` (`self.GetActorForwardVector`) AxisValue))

(event `Key|N`
  (params (Key :type "Key Structure"))
  ;[1 1 1] Note Inventory
  ;;[1 1 1] Open/close NoteInv w/ N
  (:`Pressed`
    (`self.NoteInvToggle`)))

(event `InputAxis|Look_Up/Down`
  (params (AxisValue :type "Float (single-precision)"))
  ;[1 1 1] Movement
  ;;[1 1 1] Look up/down/left/right
  (`self.AddControllerPitchInput` AxisValue))

(event `InputAxis|Left/Right`
  (params (AxisValue :type "Float (single-precision)"))
  ;[1 1 1] Movement
  ;;[1 1 1] Move for/back/left/right
  (`self.AddMovementInput` (`self.GetActorRightVector`) AxisValue))

(event `InputAction|Run`
  (params (Key :type "Key Structure"))
  (bind _charactermovement (`self.CharacterMovement`))
  ;[1 1 1] Movement
  ;;[1 1 1] Run
  (:`Pressed`
    (set `CharacterMovementComponent.MaxWalkSpeed` (`self.Run_speed`) _charactermovement))
  (:`Released`
    (set `CharacterMovementComponent.MaxWalkSpeed` 400.0 _charactermovement)))

(event `self.ReceiveActorBeginOverlap`
  (params (OtherActor :type "Actor Object Reference"))
  ;[1 1 1] "Torch" flickers and then goes out upon entering cavern
  (cast `TriggerBox` OtherActor)
  (`KismetSystemLibrary.Delay` 3.0)
  (`LightComponent.SetIntensity` (`self.PointLight`) 1000.0)
  (`KismetSystemLibrary.Delay` 0.25)
  (`KismetSystemLibrary.Delay` 0.25)
  (`LightComponent.SetIntensity` (`self.PointLight`) 750.0)
  (`LightComponent.SetIntensity` (`self.PointLight`) 1250.0)
  (`KismetSystemLibrary.Delay` 0.25)
  (`LightComponent.SetIntensity` (`self.PointLight`) 1500.0)
  (`KismetSystemLibrary.Delay` 2.0)
  (`ActorComponent.K2_DestroyComponent` (`self.PointLight`))
  (`ActorComponent.K2_DestroyComponent` (`self.Cylinder`)))

(fn `UserConstructionScript`)